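; BP_TestOBJ is a test physics object whose Cube freezes and resumes with the game's time-freeze state.
; On BeginPlay it binds CheckTimeFrozen to the time-freeze event, and that handler reads the global TimeFrozen flag.
; Freezing stores the Cube's linear and angular velocities, then disables physics simulation.
; Unfreezing reapplies the stored velocities before re-enabling simulation, with debug prints on both branches.
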(event Custom|check%20time%20frozen
  (bind _cube (Variables|Default|GetCube))
  (if (Variables|/Game/globalvariable/PDA_GlobalVariables.PDA_GlobalVariables_C|GetTimeFrozen (CallFunction|GetGlobalVariables))
    (Development|PrintString "frozen")
    (Variables|Default|Setstored%20movement%20velocity (Transformation|GetComponentVelocity _cube))
    (Variables|Default|Setstored%20rotation%20velocity (Physics|GetPhysicsAngularVelocityinDegrees _cube "None"))
    (Physics|SetSimulatePhysics (Variables|Default|GetCube) false)
    (else
      (Development|PrintString "not frozen")
      (Physics|SetPhysicsLinearVelocity (Variables|Default|GetCube) (Variables|Default|Getstored%20movement%20velocity) false "None")
      (Class|PrimitiveComponent|SetPhysicsAngularVelocityinDegrees (Variables|Default|GetCube) (Variables|Default|Getstored%20rotation%20velocity) false "None")
      (Physics|SetSimulatePhysics (Variables|Default|GetCube) true))))

(event EventBeginPlay
  (EventDispatchers|BindEventtoEHTimeFreeze (CallFunction|CheckTimeFreeze) (delegate Custom|check%20time%20frozen)))

(fn ConstructionScript)