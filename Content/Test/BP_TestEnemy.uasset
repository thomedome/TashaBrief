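; Test enemy that chases a seen player indirectly and halts while time is frozen.
; On BeginPlay it spawns a linked BP_EnemyFollowPoint and binds to the time-freeze event.
; Pawn sensing starts the follow point tracking the player, and the enemy uses AIMoveTo toward that point.
; On unfreeze it resumes moving, ramps walk speed down in a delay loop to a stop, then restores speed and forgets the player.
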(event OnSeePawn(PawnSensing)
  (params (Pawn :type Pawn%20Object%20Reference))
  (if (not (Variables|/Game/globalvariable/PDA_GlobalVariables.PDA_GlobalVariables_C|GetTimeFrozen (CallFunction|GetGlobalVariables)))
    (CallFunction|FollowPlayer)
    (Variables|Default|SetCanLoosePlayer true)
    (Variables|Default|SetHasSeenPlayer true)
    (Variables|Default|SetMoveFollowPoint true)
    (Default|FollowPlayer (Variables|Default|GetFollowPoint))))

(event Custom|FollowPlayer
  (if (not (Variables|/Game/globalvariable/PDA_GlobalVariables.PDA_GlobalVariables_C|GetTimeFrozen (CallFunction|GetGlobalVariables)))
    (AI|AIMoveTo self "0, 0, 0" (Variables|Default|GetFollowPoint) 5.0 false)))

(event Custom|check%20time%20frozen
  (if (Variables|/Game/globalvariable/PDA_GlobalVariables.PDA_GlobalVariables_C|GetTimeFrozen (CallFunction|GetGlobalVariables))
    (AI|Navigation|StopMovement (Pawn|GetController))
    (Variables|Default|SetMoveFollowPoint false)
    (elif (Variables|Default|GetHasSeenPlayer)
      (AI|AIMoveTo self "10.000000,0.000000,0.000000" (Variables|Default|GetFollowPoint) 5.0 false
        (:then
          (CallFunction|SlowtoStop))))))

(event Custom|SlowToStop
  (bind _charactermovement (Variables|Character|GetCharacterMovement))
  (if (> (Variables|/Script/Engine.CharacterMovementComponent|GetMaxWalkSpeed _charactermovement) 0.0) :!label _label
    (Variables|/Script/Engine.CharacterMovementComponent|SetMaxWalkSpeed _charactermovement (- (Variables|/Script/Engine.CharacterMovementComponent|GetMaxWalkSpeed _charactermovement) 1e+01))
    (Utilities|FlowControl|Delay 0.1)
    (goto _label)
    (else
      (AI|Navigation|StopMovement (Pawn|GetController))
      (Variables|/Script/Engine.CharacterMovementComponent|SetMaxWalkSpeed (Variables|Character|GetCharacterMovement) (Variables|Default|GetBaseMoveSpeed))
      (Variables|Default|SetHasSeenPlayer false))))

(event EventBeginPlay
  (bind _returnvalue (Transformation|GetActorTransform))
  (EventDispatchers|BindEventtoEHTimeFreeze (CallFunction|CheckTimeFreeze) (delegate Custom|check%20time%20frozen))
  (bind _returnvalue_2 (Game|SpawnActorfromClass "/Game/Test/BP_EnemyFollowPoint.BP_EnemyFollowPoint_C" (Math|Transform|MakeTransform (.location _returnvalue) (.rotation _returnvalue) "1.000000,1.000000,1.000000") "Undefined" "MultiplyWithRoot" 0 0))
  (bind _output_get (Variables|Default|SetFollowPoint _returnvalue_2))
  (Variables|/Game/Test/BP_EnemyFollowPoint.BP_EnemyFollowPoint_C|SetEnemy _output_get self))

(fn ConstructionScript)

(fn GetGlobalVariables
  (return 0))

(fn TimeFreezeToggle
  (return 0))