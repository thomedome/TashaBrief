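; Target-point actor for an enemy that tracks the player's position, with handling for time freeze.
; While the enemy allows it, FollowPlayer loops on a short delay, snapping the point to the player and orienting it along the enemy-to-point direction.
; BeginPlay binds a time-freeze event; when time is not frozen and the enemy can lose the player, the point jumps forward along that direction and clears the flag.
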(event Custom|FollowPlayer
  (if (Variables|/Game/Test/BP_TestEnemy.BP_TestEnemy_C|GetMoveFollowPoint (Variables|Default|GetEnemy)) :!label _label
    (Transformation|SetActorLocation (Transformation|GetActorLocation (Game|GetPlayerCharacter 0)) false false)
    (Transformation|SetActorRotation (Math|Rotator|FindLookatRotation (Transformation|GetActorLocation (Variables|Default|GetEnemy)) (Transformation|GetActorLocation)))
    (Utilities|FlowControl|Delay 0.25)
    (goto _label)))

(event Custom|check%20time%20frozen
  (bind _returnvalue (Transformation|GetActorForwardVector))
  (bind _enemy (Variables|Default|GetEnemy))
  (if (not (Variables|/Game/globalvariable/PDA_GlobalVariables.PDA_GlobalVariables_C|GetTimeFrozen (CallFunction|GetGlobalVariables)))
    (if (Variables|/Game/Test/BP_TestEnemy.BP_TestEnemy_C|GetCanLoosePlayer _enemy)
      (Transformation|SetActorLocation (+ (Math|Vector|MakeVector (* (.x _returnvalue) 2.5e+02) (* (.y _returnvalue) 2.5e+02) (.z _returnvalue)) (Transformation|GetActorLocation)) false false)
      (Variables|/Game/Test/BP_TestEnemy.BP_TestEnemy_C|SetCanLoosePlayer _enemy false))))

(event EventBeginPlay
  (EventDispatchers|BindEventtoEHTimeFreeze (CallFunction|CheckTimeFreeze) (delegate Custom|check%20time%20frozen)))

(fn ConstructionScript)