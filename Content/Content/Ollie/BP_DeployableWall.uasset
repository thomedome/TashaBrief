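; BP_DeployableWall is a temporary wall actor that unfolds itself on spawn, then removes itself.
; BeginPlay runs chained timelines that lower the main body, pause, slide side panels outward, raise upper panels, then shift secondary upper panels inward.
; Each stage lerps components' relative locations without sweeping and starts when the previous finishes.
; After a final delay, it spawns Niagara sparks at the main body and destroys the actor.
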(event EventBeginPlay
  (bind _alpha (Timeline|Timeline_0 PlayFromStart)
    (:Update
      (Transformation|SetRelativeLocation (Variables|Default|GetMain%20Body) (Math|Vector|Lerp(Vector) "0, 0, 0" "0.000000,0.000000,-360.000000" _alpha) false false))
    (:Finished
      (Utilities|FlowControl|Delay 1.5)
      (bind _alpha_2 (Timeline|Deploy PlayFromStart)
        (:Update
          (Transformation|SetRelativeLocation (Variables|Default|GetRight%20Wall) (Math|Vector|Lerp(Vector) "0.000000,10.000000,0.000000" "0.000000,100.000000,0.000000" _alpha_2) false false)
          (Transformation|SetRelativeLocation (Variables|Default|GetLeft%20Wall) (Math|Vector|Lerp(Vector) "0.000000,-10.000000,0.000000" "0.000000,-100.000000,0.000000" _alpha_2) false false))
        (:Finished
          (bind _alpha_3 (Timeline|Deploy%20Part%202 PlayFromStart)
            (:Update
              (Transformation|SetRelativeLocation (Variables|Default|GetLeft%20Wall%20Upper) (Math|Vector|Lerp(Vector) "0, 0, 0" "0.000000,0.000000,100.000000" _alpha_3) false false)
              (Transformation|SetRelativeLocation (Variables|Default|GetRight%20Wall%20Upper) (Math|Vector|Lerp(Vector) "0, 0, 0" "0.000000,0.000000,100.000000" _alpha_3) false false))
            (:Finished
              (bind _alpha_4 (Timeline|Timeline PlayFromStart)
                (:Update
                  (Transformation|SetRelativeLocation (Variables|Default|GetRight%20Wall%20Upper2) (Math|Vector|Lerp(Vector) "0, 0, 0" "0.000000,-40.000000,0.000000" _alpha_4) false false)
                  (Transformation|SetRelativeLocation (Variables|Default|GetLeft%20Wall%20Upper2) (Math|Vector|Lerp(Vector) "0, 0, 0" "0.000000,40.000000,0.000000" _alpha_4) false false))
                (:Finished
                  (Utilities|FlowControl|Delay 1e+01)
                  (Niagara|SpawnSystematLocation "/Game/Ollie/NS_Sparks.NS_Sparks" (Transformation|GetWorldLocation (Variables|Default|GetMain%20Body)))
                  (Actor|DestroyActor))))))))))

(fn ConstructionScript)