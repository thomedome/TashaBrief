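; BP_Grenade is a timed grenade that explodes shortly after BeginPlay and damages nearby enemies.
; After a fixed delay, a multi-sphere trace on the Visibility channel gathers hits around its Sphere component.
; Hits that cast to BP_EnemyParentOllie lose fixed health through BPCHealth.
; The NS_Explosion Niagara spawn and DestroyActor sit inside the hit loop, so neither runs when the trace returns no hits.
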(event EventBeginPlay
  (bind _sphere (Variables|Default|GetSphere))
  (bind _sphere_2 (Variables|Default|GetSphere))
  (bind _returnvalue (Transformation|GetWorldLocation _sphere))
  (Utilities|FlowControl|Delay 1.25)
  (bind _outhits (Collision|MultiSphereTraceByChannel _returnvalue _returnvalue 2.1e+02 "TraceTypeQuery1" false 0 "None"))
  (bind _array_element (Utilities|Array|ForEachLoopwithBreak _outhits)
    (:LoopBody
      (bind _asbp_enemy_parent_ollie (Utilities|Casting|CastToBP_EnemyParentOllie (.HitActor (Collision|BreakHitResult _array_element)))
        (:then
          (Default|RemoveHealth (Variables|/Game/Ollie/Enemys/BP_EnemyParentOllie.BP_EnemyParentOllie_C|GetBPC_Health _asbp_enemy_parent_ollie) 4e+01))
        (:CastFailed
          _))
      (Utilities|IsValid _sphere_2
        (:Is%20Valid
          (Niagara|SpawnSystematLocation "/Game/Ollie/NS_Explosion.NS_Explosion" (Transformation|GetWorldLocation _sphere_2)))
        (:Is%20Not%20Valid
          _))
      (Actor|DestroyActor))))

(event Collision|EventActorBeginOverlap
  (params (OtherActor :type Actor%20Object%20Reference)))

(event EventTick
  (params (DeltaSeconds :type Float%20%28single-precision%29)))

(fn ConstructionScript)