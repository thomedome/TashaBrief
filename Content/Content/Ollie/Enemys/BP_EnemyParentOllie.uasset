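; Parent enemy Blueprint that chases a sensed player and attacks in melee until killed.
; BPCHealth takes the enemy's health and armor settings and triggers a death animation, ragdoll and delayed destroy.
; PawnSensing sightings widen peripheral vision and start an AIMoveTo chase, re-issued from Tick while the seen flag holds.
; On reaching the target, a cooldown-gated montage damages the player if the Box overlap flag is set after a short delay.
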(event OnSeePawn(PawnSensing)
  (params (Pawn :type Pawn%20Object%20Reference))
  ;[0.15 0.15 0.15 0.5] If player is seen, increase vision angle and follow the player
  (Variables|Default|SetIs%20seeing%20Player true)
  (Class|PawnSensingComponent|SetPeripheralVisionAngle (Variables|Default|GetPawnSensing) 1.2e+02)
  (CallFunction|FollowPlayer))

(event OnComponentBeginOverlap(Box)
  (params (OverlappedComponent :type Primitive%20Component%20Object%20Reference) (OtherActor :type Actor%20Object%20Reference) (OtherComp :type Primitive%20Component%20Object%20Reference) (OtherBodyIndex :type Integer) (bFromSweep :type Boolean) (SweepResult :type Hit%20Result%20Structure%20%28by%20ref%29))
  ;[0.15 0.15 0.15 0.5] Melee Shabang
  (bind _output_get (Variables|Default|SetEnemy%20In%20Range true)))

(event OnComponentEndOverlap(Box)
  (params (OverlappedComponent :type Primitive%20Component%20Object%20Reference) (OtherActor :type Actor%20Object%20Reference) (OtherComp :type Primitive%20Component%20Object%20Reference) (OtherBodyIndex :type Integer))
  ;[0.15 0.15 0.15 0.5] Melee Shabang
  (Variables|Default|SetEnemy%20In%20Range false))

(event Custom|Follow%20Player
  ;[0.15 0.15 0.15 0.5] Follow The Target Player And Preform Melee Cooldown Checks
  (Variables|Default|SetCan%20Attack? true)
  (if (Variables|Default|GetIs%20seeing%20Player)
    (AI|AIMoveTo self "0, 0, 0" (stale OnSeePawn(PawnSensing) Pawn) 7e+01 false
      (:OnSuccess
        (if (Variables|Default|GetCan%20Attack?)
          (Variables|Default|SetCan%20Attack? false)
          (Utilities|FlowControl|DoOnce false :!label _label
            (:Completed
              (AI|AIMoveTo self "0, 0, 0" (stale OnSeePawn(PawnSensing) Pawn) 5e+01 false
                (:then
                  ;[0.15 0.15 0.15 0.5] Melee Shabang
                  (if (Variables|Default|GetMelee%20Toggle)
                    (Animation|PlayAnimMontage "/Game/Characters/Mannequins/Anims/Unarmed/Attack/MM_Attack_01_Montage.MM_Attack_01_Montage" 1.0 "None")
                    (Utilities|FlowControl|Delay 0.4)
                    (if (stale OnComponentBeginOverlap(Box) _output_get)
                      (Default|RemoveHealth (Variables|/Game/FirstPerson/Blueprints/BP_FirstPersonCharacter.BP_FirstPersonCharacter_C|GetBPC_Health (Variables|Default|GetPlayer%20Ref)) (Variables|Default|GetMelee%20Damage))
                      (Utilities|FlowControl|Delay 0.8)
                      (Variables|Default|SetCan%20Attack? true)
                      (goto _label Reset)
                      (else
                        (Utilities|FlowControl|Delay 0.8)
                        (Variables|Default|SetCan%20Attack? true)
                        (goto _label Reset)))))))))))
    (else
      (Variables|Default|SetIs%20seeing%20Player false))))

(event Custom|Death
  (bind _charactermovement (Variables|Character|GetCharacterMovement))
  ;[1 0.002795 4e-06 0.5] Death Event
  (Utilities|FlowControl|DoOnce false
    (:Completed
      (Variables|Default|SetCan%20Attack? false)
      (Components|Movement|StopMovementImmediately _charactermovement)
      (Variables|/Script/Engine.CharacterMovementComponent|SetMaxWalkSpeed _charactermovement 0.0)
      (Components|Animation|PlayAnimation (Variables|Character|GetMesh) "/Game/Characters/Mannequins/Anims/Death/MM_Death_Front_01.MM_Death_Front_01" false)
      (Utilities|FlowControl|Delay 1.1)
      (Physics|SetSimulatePhysics (Variables|Character|GetMesh) true)
      (Collision|SetCollisionEnabled (Variables|Collision|GetCapsuleComponent) "NoCollision")
      (Collision|SetCollisionEnabled (Variables|Character|GetMesh) "QueryAndPhysics")
      (Utilities|FlowControl|Delay 5.0)
      (Actor|DestroyActor))))

(event EventBeginPlay
  (bind _bpc_health (Variables|Default|GetBPC_Health))
  ;[0.15 0.15 0.15 0.5] Variable Setting
  (bind _returnvalue (Actor|GetActorOfClass "/Game/FirstPerson/Blueprints/BP_FirstPersonCharacter.BP_FirstPersonCharacter_C"))
  (Variables|Default|SetPlayer%20Ref _returnvalue)
  (Variables|/Game/Ollie/BPC_Health.BPC_Health_C|SetMax%20Health _bpc_health (Variables|Default|GetEnemy%20Max%20Health))
  (Variables|/Game/Ollie/BPC_Health.BPC_Health_C|SetMax%20Armor _bpc_health (Variables|Default|GetEnemy%20Max%20Armor))
  (Default|UpdateValues _bpc_health)
  (Variables|/Script/Engine.CharacterMovementComponent|SetMaxWalkSpeed (Variables|Character|GetCharacterMovement) (Variables|Default|GetMax%20Walk%20Speed))
  (EventDispatchers|BindEventtoDeath _bpc_health (delegate Custom|Death)))

(event EventTick
  (params (DeltaSeconds :type Float%20%28single-precision%29))
  ;[0.15 0.15 0.15 0.5] Check if player is sensed
  (if (Variables|Default|GetIs%20seeing%20Player)
    ;[0.15 0.15 0.15 0.5] Follow The Target Player And Preform Melee Cooldown Checks
    (if (Variables|Default|GetIs%20seeing%20Player)
      (AI|AIMoveTo self "0, 0, 0" (stale OnSeePawn(PawnSensing) Pawn) 7e+01 false
        (:OnSuccess
          (if (Variables|Default|GetCan%20Attack?)
            (Variables|Default|SetCan%20Attack? false)
            (Utilities|FlowControl|DoOnce false :!label _label
              (:Completed
                (AI|AIMoveTo self "0, 0, 0" (stale OnSeePawn(PawnSensing) Pawn) 5e+01 false
                  (:then
                    ;[0.15 0.15 0.15 0.5] Melee Shabang
                    (if (Variables|Default|GetMelee%20Toggle)
                      (Animation|PlayAnimMontage "/Game/Characters/Mannequins/Anims/Unarmed/Attack/MM_Attack_01_Montage.MM_Attack_01_Montage" 1.0 "None")
                      (Utilities|FlowControl|Delay 0.4)
                      (if (stale OnComponentBeginOverlap(Box) _output_get)
                        (Default|RemoveHealth (Variables|/Game/FirstPerson/Blueprints/BP_FirstPersonCharacter.BP_FirstPersonCharacter_C|GetBPC_Health (Variables|Default|GetPlayer%20Ref)) (Variables|Default|GetMelee%20Damage))
                        (Utilities|FlowControl|Delay 0.8)
                        (Variables|Default|SetCan%20Attack? true)
                        (goto _label Reset)
                        (else
                          (Utilities|FlowControl|Delay 0.8)
                          (Variables|Default|SetCan%20Attack? true)
                          (goto _label Reset)))))))))))
      (else
        (Variables|Default|SetIs%20seeing%20Player false)))
    (else
      (Components|Movement|StopMovementImmediately (Variables|Character|GetCharacterMovement))
      (Utilities|FlowControl|Delay 2.0)
      (Class|PawnSensingComponent|SetPeripheralVisionAngle (Variables|Default|GetPawnSensing) 6e+01))))

(fn ConstructionScript)