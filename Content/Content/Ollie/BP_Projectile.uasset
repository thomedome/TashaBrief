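; BP_Projectile is a projectile that damages an enemy and bursts into sparks on impact.
; On BeginPlay it caches the first BP_EnemyParentOllie found and keeps its sphere's collision off for a brief delay.
; On a sphere hit, only that cached enemy loses a fixed amount of health through BPCHealth, so other enemy instances take none.
; Any hit spawns NS_Sparks at the sphere and destroys the projectile.
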(event OnComponentHit(Sphere)
  (params (HitComponent :type Primitive%20Component%20Object%20Reference) (OtherActor :type Actor%20Object%20Reference) (OtherComp :type Primitive%20Component%20Object%20Reference) (NormalImpulse :type Vector :default "0, 0, 0") (Hit :type Hit%20Result%20Structure%20%28by%20ref%29))
  (bind _enemy_ref (Variables|Default|GetEnemy%20Ref))
  (if (== OtherActor _enemy_ref)
    (Default|RemoveHealth (Variables|/Game/Ollie/Enemys/BP_EnemyParentOllie.BP_EnemyParentOllie_C|GetBPC_Health _enemy_ref) 25.0))
  (Niagara|SpawnSystematLocation "/Game/Ollie/NS_Sparks.NS_Sparks" (Transformation|GetWorldLocation (Variables|Default|GetSphere)))
  (Actor|DestroyActor))

(event EventBeginPlay
  (bind _returnvalue (Actor|GetActorOfClass "/Game/Ollie/Enemys/BP_EnemyParentOllie.BP_EnemyParentOllie_C"))
  (Variables|Default|SetEnemy%20Ref _returnvalue)
  (Collision|SetCollisionEnabled (Variables|Default|GetSphere) "NoCollision")
  (Utilities|FlowControl|Delay 0.1)
  (Collision|SetCollisionEnabled (Variables|Default|GetSphere) "QueryAndPhysics"))

(event Collision|EventActorBeginOverlap
  (params (OtherActor :type Actor%20Object%20Reference)))

(event EventTick
  (params (DeltaSeconds :type Float%20%28single-precision%29)))

(fn ConstructionScript)